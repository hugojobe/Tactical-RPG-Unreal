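; Base chess piece actor handling a unit's visual feedback, HUD, passive effects and hit response.
; On spawn it applies GAS passive effects, from purchased skill-tree nodes for players or its own list for enemies.
; Timelines drive the randomized spawn scale-in, selection lift and float, and dynamic-material hit flash or death dissolve before destruction.
; Hits update GameState combat stats and RP, while the HUD reddens health when the selected unit's damage is lethal.
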(event Custom|SetIsFloating
  (params (Value :type Boolean))
  (if (!= Value (Variables|Default|GetbIsFloating))
    (bind _output_get (Variables|Default|SetbIsFloating Value))
    (if _output_get
      (bind _alpha (Timeline|FloatTimeline PlayFromStart)
        (:Update
          (Transformation|SetRelativeLocation (Variables|Default|GetUnitMeshComponent) (+ (Variables|Default|GetRelative%20Starting%20Location) (Math|Vector|Lerp(Vector) "0.000000,0.000000,50.000000" "0.000000,0.000000,75.000000" _alpha)) false false)))
      (else
        (Timeline|FloatTimeline Stop)))))

(event Custom|OnUnitHit
  (params (bWasLethal :type Boolean) (Attacker :type Chess%20Unit%20Base%20Object%20Reference) (DamageReceived :type Integer))
  (bind _returnvalue (Game|GetGameState))
  (bind _returnvalue_2 (Game|GetGameState))
  (bind _asbp_gameplay_game_state (Utilities|Casting|CastToBP_Gameplay_GameState _returnvalue))
  (bind _asbp_gameplay_game_state_2 (Utilities|Casting|CastToBP_Gameplay_GameState _returnvalue_2))
  (Utilities|FlowControl|Sequence
    (:then_0
      (if bWasLethal
        (switch Utilities|FlowControl|Switch|SwitchonEChessTeam (Variables|Default|GetTeam)
          (:Player
            (Math|Integer|IncrementInt (Variables|/Game/Blueprints/Framework/BP_Gameplay_GameState.BP_Gameplay_GameState_C|GetDeaths _asbp_gameplay_game_state_2)))
          (:Enemy
            (Math|Integer|IncrementInt (Variables|/Game/Blueprints/Framework/BP_Gameplay_GameState.BP_Gameplay_GameState_C|GetKills _asbp_gameplay_game_state_2))))))
    (:then_1
      (switch Utilities|FlowControl|Switch|SwitchonEChessTeam (Variables|Default|GetTeam)
        (:Player
          (Variables|/Game/Blueprints/Framework/BP_Gameplay_GameState.BP_Gameplay_GameState_C|SetDamageTaken _asbp_gameplay_game_state (+ (Variables|/Game/Blueprints/Framework/BP_Gameplay_GameState.BP_Gameplay_GameState_C|GetDamageTaken _asbp_gameplay_game_state) DamageReceived)))
        (:Enemy
          (Variables|/Game/Blueprints/Framework/BP_Gameplay_GameState.BP_Gameplay_GameState_C|SetDamage _asbp_gameplay_game_state (+ DamageReceived (Variables|/Game/Blueprints/Framework/BP_Gameplay_GameState.BP_Gameplay_GameState_C|GetDamage _asbp_gameplay_game_state))))))
    (:then_2
      (if (not bWasLethal)
        (Camera|PlayWorldCameraShake "/Game/Blueprints/Feedbacks/BP_HitShake.BP_HitShake_C" "0, 0, 0" 0.0 1e+04)
        (bind (_direction _emissivealpha _scalealpha) (Timeline|Hit%20Effects PlayFromStart)
          (:Update
            (Rendering|Material|SetScalarParameterValue (Variables|Default|GetUnitMaterial) "HitAlpha" _emissivealpha :!class /Script/Engine.MaterialInstanceDynamic)
            (Transformation|SetRelativeScale3D (Variables|Default|GetUnitMeshComponent) (Math|Vector|Lerp(Vector) "1.000000,1.000000,1.000000" "0.900000,0.900000,0.900000" _scalealpha))))
        (else
          (Default|AddRPPoints (.AsBP%20Gameplay%20Game%20State (Utilities|Casting|CastToBP_Gameplay_GameState (Game|GetGameState))) (Utilities|Struct|BreakUnitStats (Variables|Default|GetStats)))
          (bind (_direction_2 _dissolve _scalealpha_2) (Timeline|Death%20Effects PlayFromStart)
            (:Update
              (Rendering|Material|SetScalarParameterValue (Variables|Default|GetUnitMaterial) "DissolveAlpha" _dissolve :!class /Script/Engine.MaterialInstanceDynamic)
              (Transformation|SetRelativeScale3D (Variables|Default|GetUnitMeshComponent) (Math|Vector|Lerp(Vector) "1.000000,1.000000,1.000000" "2.000000,2.000000,2.000000" _scalealpha_2)))
            (:Finished
              (Actor|DestroyActor))))))))

(event Custom|PlaySpawnAnimation
  (Transformation|SetActorScale3D "0, 0, 0")
  (Utilities|FlowControl|Delay 1.0)
  (Components|Timeline|SetPlayRate (Variables|Default|GetSpawnTimeline) (Math|Random|RandomFloatinRange 0.35 1.0))
  (bind _alpha (Timeline|SpawnTimeline PlayFromStart)
    (:Update
      (Transformation|SetActorScale3D (Math|Vector|Lerp(Vector) "0, 0, 0" "1.000000,1.000000,1.000000" _alpha)))))

(event EventToggleUnitHUD
  (params (Visible :type Boolean) (IsEnemy :type Boolean) (SelectedInstigator :type Chess%20Unit%20Base%20Object%20Reference))
  (bind _abilitysystemcomponent (Variables|Default|GetAbilitySystemComponent))
  (bind _returnvalue (Class|AbilitySystemComponent|GetGameplayAttributeValue _abilitysystemcomponent "(AttributeName=\"Health\",Attribute=/Script/TRPG_Exam.ChessAttributeSet:Health,AttributeOwner=\"/Script/CoreUObject.Class'/Script/TRPG_Exam.ChessAttributeSet'\")"))
  (bind _returnvalue_2 (Math|Float|Truncate _returnvalue))
  (bind _unit_hud (Class|BPIUnitUI|GetUnitHUD(Message) (UserInterface|GetUserWidgetObject (Variables|Default|GetUnit%20HUD%20Widget))))
  (Utilities|IsValid SelectedInstigator
    (:Is%20Valid
      (Default|Initialize _unit_hud (Utilities|String|EnumtoString (Variables|Default|GetUnitType)) _returnvalue_2 (.MaxHP (Utilities|Struct|BreakUnitStats (Variables|Default|GetStats))) IsEnemy (and (<= _returnvalue_2 (.Damage (Utilities|Struct|BreakUnitStats (Variables|/Script/TRPG_Exam.ChessUnitBase|GetStats SelectedInstigator)))) (!= SelectedInstigator self))))
    (:Is%20Not%20Valid
      _))
  (Default|SetVisible _unit_hud Visible))

(event EventBeginPlay
  (bind _unitmeshcomponent (Variables|Default|GetUnitMeshComponent))
  (Variables|Default|SetRelative%20Starting%20Location (Variables|/Script/Engine.SceneComponent|GetRelativeLocation (Variables|Default|GetUnitMeshComponent)))
  (bind _unit_hud (Class|BPIUnitUI|GetUnitHUD(Message) (UserInterface|GetUserWidgetObject (Variables|Default|GetUnit%20HUD%20Widget))))
  (Default|Initialize _unit_hud (Utilities|String|EnumtoString (Variables|Default|GetUnitType)) 5 5 false false)
  (Default|SetVisible _unit_hud false)
  (bind _returnvalue (Rendering|Material|CreateDynamicMaterialInstance _unitmeshcomponent 0 (Rendering|Material|GetMaterial _unitmeshcomponent 0) "None" :!class /Script/Engine.PrimitiveComponent))
  (bind _output_get (Variables|Default|SetUnitMaterial _returnvalue))
  (Rendering|Material|SetMaterial _unitmeshcomponent 0 _output_get)
  (CallFunction|PlaySpawnAnimation)
  (switch Utilities|FlowControl|Switch|SwitchonEChessTeam (Variables|Default|GetTeam)
    (:Player
      (for _array_element (Class|ChessSkillTreeSubsystem|GetPurchasedPassiveNodes (Subsystems|GetChessSkillTreeSubsystem) (Variables|Default|GetUnitType))
        (GameplayEffects|ApplyGameplayEffectToSelf :self (Variables|Default|GetAbilitySystemComponent) :GameplayEffectClass (.PassiveEffect (Utilities|Struct|BreakSkillNodeData _array_element)))))
    (:Enemy
      (for _array_element_2 (Variables|Default|GetPassive%20Effect)
        (GameplayEffects|ApplyGameplayEffectToSelf :self (Variables|Default|GetAbilitySystemComponent) :GameplayEffectClass _array_element_2)))))

(event EventOnUnitClickedFeedback
  (bind _unitmeshcomponent (Variables|Default|GetUnitMeshComponent))
  (Class|ChessUnitBase|ToggleUnitHUD false false)
  (bind (_direction _floatingmovementalpha _floatingrotationalpha) (Timeline|ClickPieceTimeline Play)
    (:Update
      (Transformation|SetRelativeLocation _unitmeshcomponent (+ (Variables|Default|GetRelative%20Starting%20Location) (Math|Vector|Lerp(Vector) "0, 0, 0" "0.000000,0.000000,50.000000" _floatingmovementalpha)) false false)
      (Transformation|SetRelativeRotation _unitmeshcomponent (Math|Rotator|Lerp(Rotator) "0, 0, 0" "0.000000,0.000000,-5.000000" _floatingrotationalpha) false false))
    (:Finished
      (switch Utilities|FlowControl|Switch|SwitchonETimelineDirection _direction
        (:Forward
          (CallFunction|SetIsFloating true))))))

(event EventOnUnitUnclickedFeedback
  (bind _unitmeshcomponent (Variables|Default|GetUnitMeshComponent))
  (CallFunction|SetIsFloating false)
  (bind (_direction _floatingmovementalpha _floatingrotationalpha) (Timeline|ClickPieceTimeline Reverse)
    (:Update
      (Transformation|SetRelativeLocation _unitmeshcomponent (+ (Variables|Default|GetRelative%20Starting%20Location) (Math|Vector|Lerp(Vector) "0, 0, 0" "0.000000,0.000000,50.000000" _floatingmovementalpha)) false false)
      (Transformation|SetRelativeRotation _unitmeshcomponent (Math|Rotator|Lerp(Rotator) "0, 0, 0" "0.000000,0.000000,-5.000000" _floatingrotationalpha) false false))
    (:Finished
      (switch Utilities|FlowControl|Switch|SwitchonETimelineDirection _direction
        (:Forward
          (CallFunction|SetIsFloating true))))))

(fn ConstructionScript)

(fn GetBPChessUnit
  (return self))