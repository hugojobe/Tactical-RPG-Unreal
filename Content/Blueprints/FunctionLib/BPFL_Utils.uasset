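; Blueprint function library of display helpers for chess piece types in the game.
; GetColorByPieceType maps each of the six piece types, Pawn through King, to a fixed, muted tint.
; GetUnitIcon maps the same piece types to their matching chess icon assets.
; Both are stateless switch lookups on the piece type with hardcoded results.
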(fn GetColorbyPieceType
  (params (PieceType :type EChessUnitType%20Enum :default "Pawn"))
  (switch Utilities|FlowControl|Switch|SwitchonEChessUnitType PieceType
    (:Pawn
      (return "(R=0.287441,G=0.247961,B=0.171027,A=1.000000)"))
    (:Bishop
      (return "(R=0.181151,G=0.287441,B=0.171027,A=1.000000)"))
    (:Knight
      (return "(R=0.171027,G=0.287441,B=0.282378,A=1.000000)"))
    (:Rook
      (return "(R=0.142673,G=0.125808,B=0.287441,A=1.000000)"))
    (:Queen
      (return "(R=0.287441,G=0.171027,B=0.254037,A=1.000000)"))
    (:King
      (return "(R=0.287441,G=0.171027,B=0.171029,A=1.000000)"))))

(fn GetUnitIcon
  (params (PieceType :type EChessUnitType%20Enum :default "Pawn"))
  (switch Utilities|FlowControl|Switch|SwitchonEChessUnitType PieceType
    (:Pawn
      (return "/Game/Sprites/chess-pawn.chess-pawn"))
    (:Bishop
      (return "/Game/Sprites/chess-bishop.chess-bishop"))
    (:Knight
      (return "/Game/Sprites/chess-knight.chess-knight"))
    (:Rook
      (return "/Game/Sprites/chess-rook.chess-rook"))
    (:Queen
      (return "/Game/Sprites/chess-queen.chess-queen"))
    (:King
      (return "/Game/Sprites/chess-king.chess-king"))))