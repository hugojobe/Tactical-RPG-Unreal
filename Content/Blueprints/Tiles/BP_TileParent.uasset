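; BP_TileParent is a base tile actor that shows move or attack highlights.
; Its SetHighlight event calls the parent implementation, then reveals the move or attack highlight component, or hides both for None.
; A timeline raises the tile slightly above its stored world location when highlighted and reverses to lower it when cleared.
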(event EventSetHighlight
  (params (HighlightMode :type ETileInteraction%20Enum :default "None"))
  (|CallParentFunction HighlightMode)
  (switch Utilities|FlowControl|Switch|SwitchonETileInteraction HighlightMode
    (:None
      (Development|SetHiddeninGame (Variables|Default|GetTileHighlightMove) true true)
      (bind _alpha (Timeline|Timeline Reverse)
        (:Update
          (Transformation|SetActorLocation (+ (Variables|Default|GetTileWorldLocation) (Math|Vector|Lerp(Vector) "0, 0, 0" "0.000000,0.000000,5.000000" _alpha)) false false))))
    (:Move
      (Development|SetHiddeninGame (Variables|Default|GetTileHighlightMove) false true)
      (Timeline|Timeline Play))
    (:Attack
      (Development|SetHiddeninGame (Variables|Default|GetTileHighlightAttack) false true)
      (Timeline|Timeline Play))))

(fn ConstructionScript)