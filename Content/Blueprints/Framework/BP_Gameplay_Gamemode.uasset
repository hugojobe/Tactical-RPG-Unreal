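; Gameplay game mode for a turn-based game, extending parent turn, action and game-over handling.
; It announces each new turn and increments the game state's move counter whenever a player action finishes.
; On game over it resets time dilation, briefly waits, then shows a results modal fed with game state stats.
; Retry reloads the current level, while the Return to Camp handler is empty.
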(event Custom|OnReturnToCampClicked_Event)

(event Custom|OnRetryClicked_Event
  (bind _returnvalue (Game|GetCurrentLevelName true))
  (Game|OpenLevel(byName) (Utilities|String|StringToName _returnvalue)))

(event EventSetCurrentTurn
  (params (NewTurnState :type ETurnState%20Enum :default "Player"))
  (|CallParentFunction NewTurnState)
  (Default|CallNewTurnStarted NewTurnState))

(event EventPlayerActionFinished
  (params (Manager :type Chess%20Grid%20Manager%20Object%20Reference))
  (|CallParentFunction Manager)
  (Math|Integer|IncrementInt (Variables|/Game/Blueprints/Framework/BP_Gameplay_GameState.BP_Gameplay_GameState_C|GetMoves (.AsBP%20Gameplay%20Game%20State (Utilities|Casting|CastToBP_Gameplay_GameState (Game|GetGameState))))))

(event EventOnGameOver
  (params (WinningTeam :type EChessTeam%20Enum :default "Player") (Cause :type EGameOverCause%20Enum :default "NoPiecesRemaining"))
  (bind _returnvalue (Game|GetGameState))
  (bind _asbp_gameplay_game_state (Utilities|Casting|CastToBP_Gameplay_GameState _returnvalue))
  (|CallParentFunction WinningTeam Cause)
  (Utilities|Time|SetGlobalTimeDilation 1.0)
  (Utilities|FlowControl|Delay 0.4)
  (Utilities|FlowControl|Sequence
    (:then_0
      (bind _returnvalue_2 (UserInterface|CreateWidget "/Game/Blueprints/UI/WBP_GameOverModal.WBP_GameOverModal_C" 0 WinningTeam (Variables|/Game/Blueprints/Framework/BP_Gameplay_GameState.BP_Gameplay_GameState_C|GetCachedPlayerRpPoints _asbp_gameplay_game_state) (Variables|/Game/Blueprints/Framework/BP_Gameplay_GameState.BP_Gameplay_GameState_C|GetKills _asbp_gameplay_game_state) (Variables|/Game/Blueprints/Framework/BP_Gameplay_GameState.BP_Gameplay_GameState_C|GetDeaths _asbp_gameplay_game_state) (Variables|/Game/Blueprints/Framework/BP_Gameplay_GameState.BP_Gameplay_GameState_C|GetDamage _asbp_gameplay_game_state) (Variables|/Game/Blueprints/Framework/BP_Gameplay_GameState.BP_Gameplay_GameState_C|GetDamageTaken _asbp_gameplay_game_state) Cause (Variables|/Game/Blueprints/Framework/BP_Gameplay_GameState.BP_Gameplay_GameState_C|GetMoves _asbp_gameplay_game_state)))
      (bind _output_get (Variables|Default|SetCachedGameOverModal _returnvalue_2))
      (UserInterface|Viewport|AddtoPlayerScreen _output_get 999)
      (EventDispatchers|AssignOnReturntoCampClicked _output_get (delegate Custom|OnReturnToCampClicked_Event))
      (EventDispatchers|AssignOnRetryClicked _output_get (delegate Custom|OnRetryClicked_Event)))
    (:then_1
      (switch Utilities|FlowControl|Switch|SwitchonEChessTeam WinningTeam))))

(fn ConstructionScript)