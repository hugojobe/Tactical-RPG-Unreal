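; Player controller for gameplay that drives the game UI and a unit view camera.
; On BeginPlay it shows the mouse cursor, creates the game UI widget and finds the BP_UnitCamera actor in the level.
; Unit hover updates move that camera to a valid unit's location and forward the unit to the UI's hover widget.
; Game over only prints the winning team.
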(event Custom|OnGameOver
  (params (Winning%20Team :type EChessTeam%20Enum :default "Player"))
  (Development|PrintString (Utilities|String|Append "GAME OVER 
" (Utilities|String|EnumtoString Winning%20Team) " won") true true "(R=1.000000,G=0.000000,B=0.007502,A=1.000000)" 5e+03))

(event Custom|OnUnitHoverUpdated
  (params (Unit :type Chess%20Unit%20Base%20Object%20Reference))
  (Utilities|IsValid Unit
    (:Is%20Valid
      (Transformation|SetActorLocation (Variables|Default|GetUnitViewCamera) (Transformation|GetActorLocation Unit) false false))
    (:Is%20Not%20Valid
      _))
  (Default|OnUnitHoverUpdated (Variables|/Game/Blueprints/UI/WBP_GameUI.WBP_GameUI_C|GetWBP_UnitHover (Variables|Default|GetUI)) Unit))

(event EventBeginPlay
  (Variables|Default|SetbShowMouseCursor true)
  (bind _returnvalue (UserInterface|CreateWidget "/Game/Blueprints/UI/WBP_GameUI.WBP_GameUI_C" self))
  (bind _output_get (Variables|Default|SetUI _returnvalue))
  (UserInterface|Viewport|AddtoPlayerScreen _output_get)
  (bind _returnvalue_2 (Actor|GetActorOfClass "/Game/Blueprints/UI/BP_UnitCamera.BP_UnitCamera_C"))
  (Variables|Default|SetUnitViewCamera _returnvalue_2))

(fn ConstructionScript)