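; BP_AuraVFX is a self-contained aura feedback effect that animates a mesh's material and then removes itself.
; On BeginPlay it creates a dynamic material instance on the static mesh and runs the VFX timeline, forward or in reverse depending on PlayForward.
; The timeline drives the material's Progression and Width parameters, and the actor is destroyed when it finishes.
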(event EventBeginPlay
  (bind _returnvalue (Rendering|Material|CreateDynamicMaterialInstance (Variables|Default|GetStaticMesh) 0 (Variables|Default|GetMaterial) "None" :!class /Script/Engine.PrimitiveComponent))
  (Variables|Default|SetMat _returnvalue)
  (Rendering|Material|SetMaterial (Variables|Default|GetStaticMesh) 0 _returnvalue)
  (if (Variables|Default|GetPlayForward)
    (bind (_direction _progression_alpha _widthalpha) (Timeline|VFX PlayFromStart)
      (:Update
        (Rendering|Material|SetScalarParameterValue (Variables|Default|GetMat) "Progression" _progression_alpha :!class /Script/Engine.MaterialInstanceDynamic)
        (Rendering|Material|SetScalarParameterValue (Variables|Default|GetMat) "Width" _widthalpha :!class /Script/Engine.MaterialInstanceDynamic))
      (:Finished
        (Actor|DestroyActor)))
    (else
      (Timeline|VFX ReverseFromEnd))))

(fn ConstructionScript)