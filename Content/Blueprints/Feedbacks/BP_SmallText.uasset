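; BP_SmallText is a short-lived floating text actor that shows a message through a WBP_SmallText widget component.
; On BeginPlay it applies its Text and TextColor to the widget and records the starting transform.
; A timeline then drifts the actor a short distance from that start on all three axes, resetting rotation and scale, while animating widget opacity.
; The actor destroys itself when the timeline finishes.
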(event EventBeginPlay
  (bind _aswbp_small_text (Utilities|Casting|CastToWBP_SmallText (UserInterface|GetUserWidgetObject (Variables|Default|GetWidget))))
  (bind _output_get (Variables|Default|SetWBP _aswbp_small_text))
  (Rendering|Components|TextRender|SetText (Variables|/Game/Blueprints/UI/WBP_SmallText.WBP_SmallText_C|GetTextBlock _output_get) (Variables|Default|GetText))
  (Appearance|SetColorandOpacity (Variables|/Game/Blueprints/UI/WBP_SmallText.WBP_SmallText_C|GetTextBlock _output_get) (Utilities|Struct|MakeSlateColor (Variables|Default|GetTextColor)) :!class /Script/UMG.TextBlock)
  (Variables|Default|SetStartTransform (Transformation|GetActorTransform))
  (bind (_direction _alpha _opacityalpha) (Timeline|SmallTextTimeline Play)
    (:Update
      (Transformation|SetActorTransform (Math|Transform|MakeTransform (+ (.location (Variables|Default|GetStartTransform)) (Math|Float|Lerp 0.0 2e+01 _alpha))))
      (Widget|SetRenderOpacity (Variables|Default|GetWBP) _opacityalpha))
    (:Finished
      (Actor|DestroyActor))))

(fn ConstructionScript)